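; BP_MyActor is a practice actor that slides its static mesh back and forth along its relative X axis.
; While IsPlay is true, each Tick steps the X위치 variable one unit and applies it to the mesh, with IsMoveRight flipping just past 0 and 100.
; The step ignores delta time, so speed follows frame rate.
; BeginPlay prints a debug string; disconnected delayed-move and name-print experiments remain in the graph.
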(event EventBeginPlay
  (Development|PrintString "BEGIN PLAY"))

(event EventTick
  (params (DeltaSeconds :type Float%20%28single-precision%29))
  (if (Variables|Default|GetIsPlay)
    (if (Variables|Default|GetIsMoveRight)
      ;[1 1 1] move +
      (bind _output_get (Variables|Default|Setx위치 (+ (Variables|Default|Getx위치) 1.0)))
      (Transformation|SetRelativeLocation (Variables|Default|GetStaticMesh) (Math|Vector|MakeVector _output_get 0.0 0.0) false false)
      (if (> (Variables|Default|Getx위치) 1e+02)
        (Variables|Default|SetIsMoveRight false))
      (else
        ;[1 1 1] move -
        (bind _output_get_2 (Variables|Default|Setx위치 (+ (Variables|Default|Getx위치) -1.0)))
        (Transformation|SetRelativeLocation (Variables|Default|GetStaticMesh) (Math|Vector|MakeVector _output_get_2 0.0 0.0) false false)
        (if (< (Variables|Default|Getx위치) 0.0)
          (Variables|Default|SetIsMoveRight true))))))

(fn ConstructionScript)